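; Main character Blueprint that implements melee combat interfaces for dealing and receiving hits.
; Attacks sphere-trace at a bone socket chosen by enum and send scaled damage, with a list preventing repeat hits on one actor until a new attack clears it.
; Unblocked incoming hits trigger the hit-reaction component or set a stun type on the cached player AnimBP, which also drives finisher checks; finisher hits destroy the actor as a placeholder.
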(event `self.ReceiveBeginPlay`
  ;[0 0.6 1 0.502] BeginPlay
  (`self.GetABP`))

(event `/Game/Assets/BPI_Combat.Attack`
  (params (BoneForTrace :type "/Game/Assets/Enums/HitBoneEnum Enum" :default "NewEnumerator0") (AttackType :type "/Game/Assets/Enums/TypeOfAttackEnum Enum" :default "NewEnumerator2") (BaseDamage :type "Float (double-precision)"))
  ;[1 0 0.698 0.502] Combat Interface
  ;;[1 0 0.698 0.502] Attack Interface
  (bind _bone_name (`self.MapBoneEnumToName` BoneForTrace))
  (bind _returnvalue (`SceneComponent.GetSocketLocation` (`self.Mesh`) _bone_name))
  (bind _outhit (`KismetSystemLibrary.SphereTraceSingleForObjects` _returnvalue _returnvalue (`self.AttackRadius`) (`|MakeArray` "ObjectTypeQuery3" :!type "EObjectTypeQuery Enum")))
  (bind (_bblockinghit _binitialoverlap _time _distance _location _impactpoint _normal _impactnormal _physmat _hitactor) (`GameplayStatics.BreakHitResult` _outhit))
  (if _bblockinghit
    (if (not (`KismetArrayLibrary.Array_Contains` (`self.UnhittableEnemies`) _hitactor))
      (message `/Game/Assets/BPI_Combat.GetHit` _hitactor _outhit AttackType (* BaseDamage (`self.DamageMultiplier`)))
      (`KismetArrayLibrary.Array_Add` (`self.UnhittableEnemies`) _hitactor))))

(event `/Game/Assets/BPI_Combat.GetHit`
  (params (Hit :type "HitResult Structure") (AttackType :type "/Game/Assets/Enums/TypeOfAttackEnum Enum" :default "NewEnumerator2") (Damage :type "Float (double-precision)"))
  (bind _abp (`self.ABP`))
  ;[1 0 0.698 0.502] Combat Interface
  ;;[1 0 0.698 0.502] GetHit Interface
  (`self.EventGotHit`)
  (if (not (`BlueprintGameplayTagLibrary.HasTag` (`self.OwnedGameplayTags`) (struct :`TagName` "Combat.Blocking")))
    (switch `/Game/Assets/Enums/TypeOfAttackEnum` AttackType
      (:`NewEnumerator2`
        (`/Game/Assets/BC_HitReactions.HitReaction` (`self.BC_HitReactions`) Hit))
      (:`NewEnumerator0`
        (set `/Game/Assets/Blueprints/Character/Player/ABP_PlayerCharacter.StunType` "NewEnumerator0" _abp))
      (:`NewEnumerator1`
        (set `/Game/Assets/Blueprints/Character/Player/ABP_PlayerCharacter.StunType` "NewEnumerator1" _abp))
      (:`NewEnumerator4`
        (set `/Game/Assets/Blueprints/Character/Player/ABP_PlayerCharacter.StunType` "NewEnumerator4" _abp))
      (:`NewEnumerator3`
        ;;; Placeholder
        (`self.K2_DestroyActor`)))))

(event `/Game/Assets/BPI_Combat.NewAttack`
  ;[1 0 0.698 0.502] Combat Interface
  ;;[1 0 0.698 0.502] NewAttack Interface
  (`KismetArrayLibrary.Array_Clear` (`self.UnhittableEnemies`)))

(fn `CanFinish`
  (returns (CanFinish :type Boolean) (TypeOfFinish :type "/Game/Assets/Enums/FinisherTypeEnum Enum"))
  (locals (Finish :type "/Game/Assets/Enums/FinisherTypeEnum Enum" :default "NewEnumerator0"))
  (bind _abp (`self.ABP`))
  (bind _finish (`local.Finish`))
  (bind _stuntype (`/Game/Assets/Blueprints/Character/Player/ABP_PlayerCharacter.StunType` _abp))
  (`KismetSystemLibrary.PrintString` (`|GetEnumeratorNameAsString` _stuntype))
  (switch `/Game/Assets/Enums/TypeOfAttackEnum` _stuntype
    (:`NewEnumerator2`
      _)
    (:`NewEnumerator0`
      (set `local.Finish` "NewEnumerator0"))
    (:`NewEnumerator1`
      (set `local.Finish` "NewEnumerator1" :!label _label))
    (:`NewEnumerator4`
      (goto _label))
    (:`NewEnumerator3`
      _))
  (`KismetSystemLibrary.PrintString` (`|GetEnumeratorNameAsString` _finish))
  (return (`/Game/Assets/Blueprints/Character/Player/ABP_PlayerCharacter.isFinishable` _abp) _finish))

(fn `GetABP`
  (bind _asabp_player_character (cast `/Game/Assets/Blueprints/Character/Player/ABP_PlayerCharacter` (`SkeletalMeshComponent.GetAnimInstance` (`self.Mesh`))))
  (set `self.ABP` _asabp_player_character))

(fn `GetDirectionEnum`
  (params (X :type "Float (double-precision)") (Y :type "Float (double-precision)"))
  (returns (Direction :type "/Game/Assets/Enums/MoveDirectionEnum Enum"))
  (locals (InputAttackType :type "/Game/Assets/Enums/MoveDirectionEnum Enum"))
  (if (> (`KismetMathLibrary.Abs` X) (`KismetMathLibrary.Abs` Y))
    (if (> X 0.0)
      (set `local.InputAttackType` "NewEnumerator3")
      (else
        (set `local.InputAttackType` "NewEnumerator2")))
    (elif (> Y 0.0)
      (set `local.InputAttackType` "NewEnumerator0")
      (else
        (set `local.InputAttackType` "NewEnumerator1"))))
  (return (`local.InputAttackType`)))

(fn `IsAttacking`
  (returns (IsAttacking :type Boolean))
  (return (`/Game/Assets/Blueprints/Character/Player/ABP_PlayerCharacter.IsAttacking` (`self.ABP`))))

(fn `MapBoneEnumToName`
  (params (`Hit with what bone` :type "/Game/Assets/Enums/HitBoneEnum Enum" :default "NewEnumerator0"))
  (returns (`Bone name` :type Name))
  (locals (Bone :type Name))
  (switch `/Game/Assets/Enums/HitBoneEnum` `Hit with what bone`
    (:`NewEnumerator0`
      (set `local.Bone` "hand_l"))
    (:`NewEnumerator1`
      (set `local.Bone` "hand_r"))
    (:`NewEnumerator2`
      (set `local.Bone` "foot_l"))
    (:`NewEnumerator3`
      (set `local.Bone` "foot_r"))
    (:`NewEnumerator4`
      (set `local.Bone` "head")))
  (return (`local.Bone`)))

(fn `UserConstructionScript`)